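; Shotgun weapon Blueprint that supplies the hit detection for firing.
; The WeaponTrace event runs a single thin CameraTrace with a fixed range and persistent debug drawing, with no pellet spread.
; If the hit actor implements BPI_Damage, it receives a TakeDamage interface message, so the shotgun needs no knowledge of the target's class.
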(event EventBeginPlay
  (|CallParentFunction) ; This node is disabled and will not be called.\nDrag off pins to build functionality.
)

(event Collision|EventActorBeginOverlap
  (params (OtherActor :type Actor%20Object%20Reference))
  (|CallParentFunction OtherActor) ; This node is disabled and will not be called.\nDrag off pins to build functionality.
)

(event EventTick
  (params (DeltaSeconds :type Float%20%28single-precision%29))
  (|CallParentFunction DeltaSeconds) ; This node is disabled and will not be called.\nDrag off pins to build functionality.
)

(event EventWeaponTrace
  (bind _outhit (CallFunction|CameraTrace 5e+03 1.0 "Persistent"))
  (if (Utilities|DoesObjectImplementInterface (.HitActor (Collision|BreakHitResult _outhit)) "/Game/MyGame/Blueprints/BPI_Damage.BPI_Damage_C")
    (Class|BPIDamage|TakeDamage(Message) (.HitActor (Collision|BreakHitResult _outhit)))))

(fn ConstructionScript
  (|CallParentFunction))