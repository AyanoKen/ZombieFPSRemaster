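; Base weapon actor that handles firing, ammo, reloading and a zoom FOV multiplier through Blueprint interface calls.
; Firing spends a round, spawns muzzle particles and sound at the Arrow, then calls WeaponTrace, an empty event here.
; An empty magazine or reload call enters a DoOnce-guarded reload that shows a timed progress widget and refills ammo after a delay.
; The WeaponSpeed delay ends the fire chain without gating later shots.
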(event Custom|ReloadWeapon
  (Utilities|FlowControl|DoOnce false :!label _label
    (:Completed
      (bind _returnvalue (UserInterface|CreateWidget "/Game/MyGame/UI/WB_ReloadBar.WB_ReloadBar_C"))
      (Default|ReloadAnimation _returnvalue (Variables|ShootParams|GetReloadTime))
      (UserInterface|Viewport|AddtoViewport _returnvalue 0)
      (Utilities|FlowControl|Delay (Variables|ShootParams|GetReloadTime))
      (Variables|Ammo|SetCurrentAmmo (Variables|Ammo|GetMaxAmmo))
      (goto _label))))

(event Custom|WeaponTrace)

(event EventBeginPlay
  (Variables|Ammo|SetCurrentAmmo (Variables|Ammo|GetMaxAmmo)))

(event Collision|EventActorBeginOverlap
  (params (OtherActor :type Actor%20Object%20Reference)))

(event EventTick
  (params (DeltaSeconds :type Float%20%28single-precision%29)))

(event EventBPIReloadWeapon
  (Utilities|FlowControl|DoOnce false :!label _label
    (:Completed
      (bind _returnvalue (UserInterface|CreateWidget "/Game/MyGame/UI/WB_ReloadBar.WB_ReloadBar_C"))
      (Default|ReloadAnimation _returnvalue (Variables|ShootParams|GetReloadTime))
      (UserInterface|Viewport|AddtoViewport _returnvalue 0)
      (Utilities|FlowControl|Delay (Variables|ShootParams|GetReloadTime))
      (Variables|Ammo|SetCurrentAmmo (Variables|Ammo|GetMaxAmmo))
      (goto _label))))

(event EventBPIFireWeapon
  (if (<= (Variables|Ammo|GetCurrentAmmo) 0)
    (CallFunction|ReloadWeapon)
    (else
      (Variables|Ammo|SetCurrentAmmo (- (Variables|Ammo|GetCurrentAmmo) 1))
      (Development|PrintString "Shooting")
      (CallFunction|WeaponEffects)
      (CallFunction|WeaponTrace)
      (Utilities|FlowControl|Delay (Variables|Default|GetWeaponSpeed)))))

(fn ConstructionScript)

(fn WeaponEffects
  (bind _arrow (Variables|Default|GetArrow))
  (bind _returnvalue (Transformation|GetWorldTransform _arrow))
  (Effects|SpawnEmitteratLocation (Variables|WeaponEffects|GetWeaponFireEffect) (.location _returnvalue) (.rotation _returnvalue) (Variables|WeaponEffects|GetWeaponFireEffectScale))
  (Audio|SpawnSoundatLocation (Variables|WeaponEffects|GetWeaponFireSound) (.location _returnvalue) "0, 0, 0" 1.0 1.0 0.0 0 0)
  (return))

(fn BPIGetZoom
  (return (Variables|Default|GetFOVMultiplier)))