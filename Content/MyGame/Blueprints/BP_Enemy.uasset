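; BP_Enemy is a melee-style enemy that chases the player on sight and dies when its HP runs out.
; PawnSensing sets a seen flag, never cleared here, and triggers an AI MoveTo toward the first player character.
; On arrival it plays an attack montage, using the returned montage length as the delay before it can attack again.
; Incoming damage lowers EnemyHP and destroys the actor at zero; the attack itself applies no damage in this graph.
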(event OnSeePawn(PawnSensing)
  (params (Pawn :type Pawn%20Object%20Reference))
  (Variables|Default|SetisSeeingPlayer? true)
  (CallFunction|FollowPlayer))

(event Custom|FollowPlayer
  (if (Variables|Default|GetisSeeingPlayer?)
    (AI|AIMoveTo self "0, 0, 0" (Game|GetPlayerCharacter 0) 1e+01 false
      (:OnSuccess
        (if (Variables|Default|GetcanAttack?)
          (Variables|Default|SetcanAttack? false)
          (bind _returnvalue (Animation|PlayAnimMontage "/Game/MyGame/Animation/AnimMontage_DemiDevi.AnimMontage_DemiDevi" 1.0 "None"))
          (Utilities|FlowControl|Delay _returnvalue)
          (Variables|Default|SetcanAttack? true))))))

(event EventBeginPlay)

(event Collision|EventActorBeginOverlap
  (params (OtherActor :type Actor%20Object%20Reference)))

(event EventTick
  (params (DeltaSeconds :type Float%20%28single-precision%29)))

(event EventTakeDamage
  (params (Damage :type Integer))
  (Variables|Default|SetEnemyHP (- (Variables|Default|GetEnemyHP) Damage))
  (if (<= (Variables|Default|GetEnemyHP) 0)
    (Actor|DestroyActor)))

(fn ConstructionScript)