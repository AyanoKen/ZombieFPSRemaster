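; Boss enemy that chases the player, attacks with montages and dies when its HP runs out.
; Pawn sensing sets a blackboard chase flag on its AI controller when it sees the first-person character.
; AttackPlayer plays a random montage gated by CanAttack, then damages the player after a delay of the montage's length, with no range check.
; TakeDamage reduces HP and, at zero, plays the death montage before destroying the actor.
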(event OnSeePawn(PawnSensing)
  (params (Pawn :type Pawn%20Object%20Reference))
  (Utilities|Casting|CastToBP_FirstPersonCharacter Pawn)
  (AI|Components|Blackboard|SetValueasBool (AI|GetBlackboard (AI|GetAIController self)) (Utilities|Name|MakeLiteralName "ChasingPlayer?") true))

(event Custom|AttackPlayer
  (bind _returnvalue (CallFunction|AttackAnim))
  (Utilities|FlowControl|Delay _returnvalue)
  (Variables|Default|SetcanAttack? true)
  (Class|BPIDamage|TakeDamage(Message) (Game|GetPlayerCharacter 0) (Variables|EnemyStats|GetEnemyDamage)))

(event EventBeginPlay
  (Variables|/Script/Engine.CharacterMovementComponent|SetMaxWalkSpeed (Variables|Character|GetCharacterMovement) (Variables|Animation|GetMovementSpeed)))

(event Collision|EventActorBeginOverlap
  (params (OtherActor :type Actor%20Object%20Reference)))

(event EventTick
  (params (DeltaSeconds :type Float%20%28single-precision%29)))

(event EventTakeDamage
  (params (Damage :type Integer))
  (bind _output_get (Variables|EnemyStats|SetEnemyHP (- (Variables|EnemyStats|GetEnemyHP) Damage)))
  (if (<= _output_get 0)
    (bind _returnvalue (Animation|PlayAnimMontage (Variables|Animation|GetDeathMontage) 1.0 "None"))
    (Utilities|FlowControl|Delay _returnvalue)
    (Actor|DestroyActor)))

(fn ConstructionScript)

(fn AttackAnim
  (if (Variables|Default|GetcanAttack?)
    (Variables|Default|SetcanAttack? false)
    (bind _returnvalue (Animation|PlayAnimMontage (Utilities|Array|Get(acopy) (Variables|Animation|GetAttackMontage) (Math|Random|RandomIntegerinRange 0 (Utilities|Array|Length (Variables|Animation|GetAttackMontage)))) 1.0 "None"))
    (return _returnvalue)))